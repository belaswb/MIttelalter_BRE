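; A survival game mode that drains Hunger and Thirst values over time.
; On BeginPlay it adds the GameUi widget to the viewport and, if the player character is a MyPLayer, starts an endless Delay loop with random intervals of a few seconds.
; Each pass subtracts random amounts from both values, using larger ranges when Hardcore is set, with no clamping.
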(event `Thirst?`
  (if (`self.Hardcore`)
    (set `self.Thirst` (- (`self.Thirst`) (`KismetMathLibrary.RandomFloatInRange` 0.07 0.4)))
    (else
      (set `self.Thirst` (- (`self.Thirst`) (`KismetMathLibrary.RandomFloatInRange` 0.04 0.1))))))

(event `Hungry`
  (if (`self.Hardcore`)
    (set `self.Hunger` (- (`self.Hunger`) (`KismetMathLibrary.RandomFloatInRange` 0.05 0.1)))
    (else
      (set `self.Hunger` (- (`self.Hunger`) (`KismetMathLibrary.RandomFloatInRange` 0.01 0.05))))))

(event `self.ReceiveBeginPlay`
  (`|ExecutionSequence`
    (:`then_0`
      (bind _returnvalue (`|CreateWidget` "/Game/Ui/GameUi.GameUi_C"))
      (`UserWidget.AddToViewport` _returnvalue 0))
    (:`then_1`
      (cast `/Game/Blueprints/MyPLayer` (`GameplayStatics.GetPlayerCharacter` 0))
      (`self.Thirst?` :!label _label)
      (`self.Hungry`)
      (`KismetSystemLibrary.Delay` (`KismetMathLibrary.RandomFloatInRange` 1.0 5.0))
      (goto _label))))

(fn `UserConstructionScript`)