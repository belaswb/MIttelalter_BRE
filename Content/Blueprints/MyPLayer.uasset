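; Third-person player character for a shooter, handling movement, sprint, aim and shoulder camera timelines, pause menu and inventory.
; Number keys toggle spawning a Scar or AK47 on the weapon socket, with delay-looped automatic fire and montage-driven reload per gun slot.
; A forward line trace drives interaction with items, heal pickups, backpacks and vehicle possession.
; Healing uses a hold-input macro, consumes a GameMode heal item and locks input during its montage.
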(event `InputAction|Reload`
  (params (Key :type "Key Structure"))
  ;[1 1 1] Reload
  (:`Pressed`
    (`self.Reload`)))

(event `InputAction|Heal`
  (params (Key :type "Key Structure"))
  ;[1 1 1] Healing
  (:`Pressed`
    (`self.HoldInput` 1.0
      (:`Held`
        (`self.HealingPlayer`)
        (`KismetSystemLibrary.Delay` 3.27)
        (`self.EnableInput` (`GameplayStatics.GetPlayerController` 0))))))

(event `Reload`
  (bind _charactermovement (`self.CharacterMovement`))
  ;[1 1 1] Reload
  (if (`self.Equipt`)
    (`/Engine/EditorBlueprintResources/StandardMacros.DoOnce` false :!label _label
      (:`Completed`
        (set `CharacterMovementComponent.MaxWalkSpeed` 0.0 _charactermovement)
        (`self.PlayAnimMontage` "/Game/Animation/MainCharacter/Rifle/Reloading_Montage.Reloading_Montage")
        (`KismetSystemLibrary.Delay` 3.3)
        (switch `/Game/Blueprints/Guns/Weapon` (`self.Gun`)
          (:`NewEnumerator0`
            (bind _output_get (set `self.MagAmmo` 30))
            (set `self.Ammo` (- (`self.Ammo`) _output_get)))
          (:`NewEnumerator1`
            (bind _output_get_2 (set `self.MagAmmo2` 35))
            (set `self.Ammo` (- _output_get_2 (`self.MagAmmo2`)))))
        (set `CharacterMovementComponent.MaxWalkSpeed` 200.0 _charactermovement)
        (goto _label :!via `Reset`)))))

(event `self.ReceiveTick`
  (params (DeltaSeconds :type "Float (single-precision)"))
  (`KismetSystemLibrary.PrintString` (`|GetEnumeratorNameAsString` (`self.Gun`))))

(event `Key|Escape` :paused true
  (params (Key :type "Key Structure"))
  (bind _returnvalue (`GameplayStatics.GetPlayerController` 0))
  (bind _pausemenu (`self.Pausemenu`))
  (:`Pressed`
    (`/Engine/EditorBlueprintResources/StandardMacros.IsValid` (`self.Pausemenu`)
      (:`Is Valid`
        _)
      (:`Is Not Valid`
        (bind _returnvalue_2 (`|CreateWidget` "/Game/Ui/Pause.Pause_C"))
        (set `self.Pausemenu` _returnvalue_2)))
    (if (`GameplayStatics.IsGamePaused`)
      (`WidgetLayoutLibrary.RemoveAllWidgets`)
      (bind _returnvalue_3 (`|CreateWidget` "/Game/Ui/GameUi.GameUi_C"))
      (`UserWidget.AddToViewport` _returnvalue_3 0)
      (`GameplayStatics.SetGamePaused` false)
      (set `PlayerController.bShowMouseCursor` false _returnvalue)
      (`WidgetBlueprintLibrary.SetInputMode_GameOnly` _returnvalue)
      (else
        (`UserWidget.AddToViewport` _pausemenu 0)
        (`GameplayStatics.SetGamePaused` true)
        (set `PlayerController.bShowMouseCursor` true _returnvalue)
        (`WidgetBlueprintLibrary.SetInputMode_GameAndUIEx` _returnvalue _pausemenu "LockInFullscreen")))))

(event `InputAction|Fire`
  (params (Key :type "Key Structure"))
  (bind _magammo (`self.MagAmmo`))
  (bind _as_rilfe_master (`self.As Rilfe Master`))
  (bind _magammo2 (`self.MagAmmo2`))
  (:`Pressed`
    (bind _output_get (set `self.Fire?` true))
    ;[1 1 1] Fire
    (if _output_get :!label _label_2
      (switch `/Game/Blueprints/Guns/Weapon` (`self.Gun`)
        (:`NewEnumerator0`
          (if (not (< _magammo 0))
            (set `self.MagAmmo` (- _magammo 1))
            (`/Game/Blueprints/Guns/RilfeMaster.Fire` _as_rilfe_master)
            (`KismetSystemLibrary.Delay` 0.1)
            (goto _label_2)))
        (:`NewEnumerator1`
          (if (not (< _magammo2 0))
            (set `self.MagAmmo2` (- _magammo2 1))
            (`/Game/Blueprints/Guns/RilfeMaster.Fire` _as_rilfe_master)
            (`KismetSystemLibrary.Delay` 0.3)
            (goto _label_2))))))
  (:`Released`
    (set `self.Fire?` false)))

(event `InputAction|OpenInv`
  (params (Key :type "Key Structure"))
  (bind _inventory_window (`self.Inventory_Window`))
  (bind _canvaspanel_0 (`/Game/Ui/Inventory/inventorywindow.CanvasPanel_0` _inventory_window))
  ;[1 1 1] Open Inventory
  (:`Pressed`
    (if (`/Game/Ui/Inventory/inventorywindow.InventoryOpen` _inventory_window)
      (`Widget.SetVisibility` _canvaspanel_0 "Hidden")
      (set `/Game/Ui/Inventory/inventorywindow.InventoryOpen` false _inventory_window)
      (else
        (`Widget.SetVisibility` _canvaspanel_0 "Visible")
        (set `/Game/Ui/Inventory/inventorywindow.InventoryOpen` true _inventory_window)))
    (`/Game/Ui/Inventory/inventorywindow.RenderInvenory` _inventory_window (`self.Inventory`))))

(event `InputAction|Interact`
  (params (Key :type "Key Structure"))
  (:`Pressed`
    (bind _outhit (`self.LineTraceByChannel`))
    (`|ExecutionSequence`
      (:`then_0`
        (bind (_bblockinghit _binitialoverlap _time _distance _location _impactpoint _normal _impactnormal _physmat _hitactor) (`GameplayStatics.BreakHitResult` _outhit))
        (bind _asitem_master (cast `/Game/Blueprints/Items/Master/ItemMaster` _hitactor))
        (message `/Game/Blueprints/Items/Interact.Interact` _asitem_master))
      (:`then_1`
        (bind _asheal_master (cast `/Game/Blueprints/Items/Master/Heal_Master` _hitactor))
        (`/Game/Blueprints/Items/Master/Heal_Master.Item More` _asheal_master))
      (:`then_2`
        (bind _asbackpack (cast `/Game/Blueprints/Items/Backpack` _hitactor))
        (`self.TakeBackpack`)
        (`self.K2_DestroyActor` _asbackpack))
      (:`then_3`
        (`self.EnterCar` _outhit)))))

(event `InputAxis|Look Up`
  (params (AxisValue :type "Float (single-precision)"))
  (`self.AddControllerYawInput` AxisValue))

(event `InputAction|Aim`
  (params (Key :type "Key Structure"))
  ;[1 1 1] Aim
  (:`Pressed`
    (set `self.Aim?` true)
    (bind (_direction _newtrack_0) (`Timeline|Timeline_0` :!label _label_3)
      (:`Update`
        (set `SpringArmComponent.TargetArmLength` _newtrack_0 (`self.SpringArm`)))))
  (:`Released`
    (set `self.Aim?` false)
    (goto _label_3 :!via `Reverse`)))

(event `InputAxis|LookRight`
  (params (AxisValue :type "Float (single-precision)"))
  (`self.AddControllerPitchInput` AxisValue))

(event `InputAxis|MoveForward`
  (params (AxisValue :type "Float (single-precision)"))
  (bind (_returnvalue_roll _returnvalue_pitch _returnvalue_yaw) (`KismetMathLibrary.BreakRotator` (`self.GetControlRotation`)))
  ;[1 1 1] Movement
  (`self.AddMovementInput` (`KismetMathLibrary.GetForwardVector` (`KismetMathLibrary.MakeRotator` 0.0 0.0 _returnvalue_yaw)) AxisValue))

(event `InputAxis|Right`
  (params (AxisValue :type "Float (single-precision)"))
  (bind (_returnvalue_roll _returnvalue_pitch _returnvalue_yaw) (`KismetMathLibrary.BreakRotator` (`self.GetControlRotation`)))
  ;[1 1 1] Movement
  (`self.AddMovementInput` (`KismetMathLibrary.GetRightVector` (`KismetMathLibrary.MakeRotator` 0.0 0.0 _returnvalue_yaw)) AxisValue))

(event `InputAction|Jogg`
  (params (Key :type "Key Structure"))
  (bind _charactermovement (`self.CharacterMovement`))
  ;[1 1 1] Jogg
  (:`Pressed`
    (set `self.Sprint?` true)
    (if (`self.Equipt`)
      (set `CharacterMovementComponent.MaxWalkSpeed` 400.0 _charactermovement)
      (else
        (set `CharacterMovementComponent.MaxWalkSpeed` 350.0 _charactermovement))))
  (:`Released`
    (set `self.Sprint?` false)
    (set `CharacterMovementComponent.MaxWalkSpeed` 200.0 _charactermovement)))

(event `InputAction|Switch left`
  (params (Key :type "Key Structure"))
  ;[1 1 1] Switch Cam
  (:`Pressed`
    (bind (_direction _newtrack_0) (`Timeline|Timeline_1` :!label _label_4)
      (:`Update`
        (`SceneComponent.K2_SetRelativeLocation` (`self.SpringArm`) (`KismetMathLibrary.MakeVector` 0.0 _newtrack_0 80.0) false false)))))

(event `Key|One`
  (params (Key :type "Key Structure"))
  (bind _as_rilfe_master (`self.As Rilfe Master`))
  ;[1 1 1] Weapon
  (:`Pressed`
    (set `self.Gun` "NewEnumerator0")
    (`/Engine/EditorBlueprintResources/StandardMacros.IsValid` _as_rilfe_master
      (:`Is Valid`
        (`self.K2_DestroyActor` _as_rilfe_master))
      (:`Is Not Valid`
        _))
    (`/Engine/EditorBlueprintResources/StandardMacros.FlipFlop`
      (:`A`
        (set `self.Equipt` true)
        (`/Engine/EditorBlueprintResources/StandardMacros.IsValid` (stale `Key|Two` _output_get)
          (:`Is Valid`
            (`self.K2_DestroyActor` (stale `Key|Two` _output_get))
            (switch `/Game/Blueprints/Guns/Weapon` "NewEnumerator0"
              (:`NewEnumerator0`
                _)))
          (:`Is Not Valid`
            _))
        (bind _output_get (`self.Weapon`))
        (bind _asbackpack (cast `/Game/Blueprints/Items/Backpack` (`GameplayStatics.GetPlayerPawn` 0)))
        (`SceneComponent.SetVisibility` (`/Game/Blueprints/Items/Backpack.RilfeMaster` _asbackpack) false false))
      (:`B`
        (set `self.Equipt` false)))))

(event `InputAction|Switch Right`
  (params (Key :type "Key Structure"))
  ;[1 1 1] Switch Cam
  (:`Pressed`
    (goto _label_4 :!via `Reverse`)))

(event `Key|Two`
  (params (Key :type "Key Structure"))
  (bind _as_rilfe_master (`self.As Rilfe Master`))
  ;[1 1 1] Weapon
  (:`Pressed`
    (set `self.Gun` "NewEnumerator1")
    (`/Engine/EditorBlueprintResources/StandardMacros.IsValid` _as_rilfe_master
      (:`Is Valid`
        (`self.K2_DestroyActor` _as_rilfe_master))
      (:`Is Not Valid`
        _))
    (`/Engine/EditorBlueprintResources/StandardMacros.FlipFlop`
      (:`A`
        (set `self.Equipt` true)
        (`/Engine/EditorBlueprintResources/StandardMacros.IsValid` (stale `Key|One` _output_get)
          (:`Is Valid`
            (`self.K2_DestroyActor` (stale `Key|One` _output_get))
            (switch `/Game/Blueprints/Guns/Weapon` "NewEnumerator1"
              (:`NewEnumerator1`
                _)))
          (:`Is Not Valid`
            _))
        (bind _output_get (`self.Weapon_2`))
        (bind _asbackpack (cast `/Game/Blueprints/Items/Backpack` (`GameplayStatics.GetPlayerPawn` 0)))
        (`SceneComponent.SetVisibility` (`/Game/Blueprints/Items/Backpack.RilfeMaster1` _asbackpack) false false))
      (:`B`
        (set `self.Equipt` false)))))

(fn `EnterCar`
  (params (Hit :type "HitResult Structure (by ref)"))
  (bind _asmaster_vehicle (cast `/Game/Blueprints/Vehicle/MasterVehicle` (`.HitActor` (`GameplayStatics.BreakHitResult` Hit))))
  (`Controller.Possess` (`GameplayStatics.GetPlayerController` 0) _asmaster_vehicle)
  (`self.K2_AttachToActor` self null "None" "SnapToTarget" "SnapToTarget" "SnapToTarget" true)
  (`SceneComponent.SetVisibility` (`self.Mesh`) false false)
  (`PrimitiveComponent.SetCollisionEnabled` (`self.CapsuleComponent`) "NoCollision")
  (message `/Game/Blueprints/BPI_Character.EnterCar` _asmaster_vehicle self)
  (`SceneComponent.SetVisibility` (`/Game/Blueprints/Vehicle/MasterVehicle.SkeletalMesh` _asmaster_vehicle) true false))

(fn `GetWeaponSocket`
  (params (SocketName :type Name :default "None"))
  (returns (SocketTransform :type "Transform Structure")))

(fn `HealingPlayer`
  (bind _asnew_game_mode (cast `/Game/Blueprints/NewGameMode` (`GameplayStatics.GetGameMode`)))
  (set `self.As New Game Mode` _asnew_game_mode)
  (bind _heal_item (`/Game/Blueprints/NewGameMode.Heal_item` _asnew_game_mode))
  (if (not (<= _heal_item 0))
    (set `/Game/Blueprints/NewGameMode.Heal_item` (- _heal_item 1) _asnew_game_mode)
    (`self.DisableInput` (`GameplayStatics.GetPlayerController` 0))
    (`self.PlayAnimMontage` "/Game/Animation/MainCharacter/Heal/Kick_To_The_Groin_Montage.Kick_To_The_Groin_Montage")
    (return)))

(fn `LineTraceByChannel`
  (returns (OutHit :type "HitResult Structure"))
  (bind _scene (`self.Scene`))
  (bind _returnvalue (`SceneComponent.K2_GetComponentLocation` _scene))
  (bind _outhit (`KismetSystemLibrary.LineTraceSingle` :`Start` _returnvalue :`End` (+ _returnvalue (* (`SceneComponent.GetForwardVector` _scene) 500.0)) :`TraceChannel` "TraceTypeQuery1" :`DrawDebugType` "ForDuration"))
  (return _outhit))

(fn `TakeBackpack`
  (bind _returnvalue (`|SpawnActorFromClass` "/Game/Blueprints/Items/Backpack.Backpack_C" (`self.GetTransform`) "Undefined" "OverrideRootScale" null null))
  (bind _output_get (set `self.As Backpack` _returnvalue))
  (`SceneComponent.K2_AttachToComponent` (`Actor.RootComponent` _output_get) (`self.Mesh`) "Backpack" "SnapToTarget" "SnapToTarget" "SnapToTarget" true)
  (`PrimitiveComponent.SetCollisionEnabled` (`/Game/Blueprints/Items/Backpack.SM_PickUp_Bag_03` _output_get) "NoCollision"))

(fn `UserConstructionScript`)

(fn `Weapon`
  (returns (Output_Get :type "/Game/Blueprints/Guns/RilfeMaster Object Reference"))
  (bind _returnvalue (`|SpawnActorFromClass` "/Game/Blueprints/Guns/Scar.Scar_C" (`self.GetTransform`) "Undefined" "OverrideRootScale" null null))
  (bind _output_get (set `self.As Rilfe Master` _returnvalue))
  (`SceneComponent.K2_AttachToComponent` (`Actor.RootComponent` _output_get) (`self.Mesh`) "Weapon" "SnapToTarget" "SnapToTarget" "SnapToTarget" true)
  (return _output_get))

(fn `Weapon_2`
  (returns (Output_Get :type "/Game/Blueprints/Guns/RilfeMaster Object Reference"))
  (bind _returnvalue (`|SpawnActorFromClass` "/Game/Blueprints/Guns/Ak47.Ak47_C" (`self.GetTransform`) "Undefined" "OverrideRootScale" null null))
  (bind _output_get (set `self.As Rilfe Master` _returnvalue))
  (`SceneComponent.K2_AttachToComponent` (`Actor.RootComponent` _output_get) (`self.Mesh`) "Weapon" "SnapToTarget" "SnapToTarget" "SnapToTarget" true)
  (return _output_get))