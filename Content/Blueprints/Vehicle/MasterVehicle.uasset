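; Base drivable vehicle pawn that the player enters and exits, with throttle, steering, handbrake and camera look input feeding the controller and VehicleMovement.
; EnterCar stores the Player; Interact re-possesses it, restores collision, detaches it at the Scene component's location and copies its mesh onto a visible SkeletalMesh.
; Light input toggles spot and point lights, while holding S fades two other point lights through a reversible Timeline.
; GetWeaponSocket is an empty stub.
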(event `InputAxis|Look Up`
  (params (AxisValue :type "Float (single-precision)"))
  (`self.AddControllerYawInput` AxisValue))

(event `InputAction|Handbreak`
  (params (Key :type "Key Structure"))
  (bind _vehiclemovement (`self.VehicleMovement`))
  (:`Pressed`
    (`WheeledVehicleMovementComponent.SetHandbrakeInput` _vehiclemovement true))
  (:`Released`
    (`WheeledVehicleMovementComponent.SetHandbrakeInput` _vehiclemovement false)))

(event `/Game/Blueprints/BPI_Character.EnterCar`
  (params (Player :type "Character Object Reference"))
  (set `self.Player` Player))

(event `InputAxis|LookRight`
  (params (AxisValue :type "Float (single-precision)"))
  (`self.AddControllerPitchInput` AxisValue))

(event `InputAction|Interact`
  (params (Key :type "Key Structure"))
  (bind _skeletalmesh (`self.SkeletalMesh`))
  (bind _player (`self.Player`))
  (:`Pressed`
    (`Controller.Possess` (`GameplayStatics.GetPlayerController` 0) _player)
    (`PrimitiveComponent.SetCollisionEnabled` (`Character.CapsuleComponent` _player) "QueryAndPhysics")
    (`SceneComponent.K2_SetWorldLocation` (`Character.CapsuleComponent` (`self.Player`)) (`SceneComponent.K2_GetComponentLocation` (`self.Scene`)) false false)
    (`self.K2_DetachFromActor` _player "KeepWorld" "KeepWorld" "KeepWorld")
    (`SkinnedMeshComponent.SetSkinnedAssetAndUpdate` _skeletalmesh (`SkinnedMeshComponent.SkeletalMesh` (`Character.Mesh` (`self.Player`))) true)
    (`SceneComponent.SetVisibility` _skeletalmesh true false)
    (`SceneComponent.SetVisibility` (`Character.Mesh` _player) true false)))

(event `InputAction|Light`
  (params (Key :type "Key Structure"))
  (:`Pressed`
    (`/Engine/EditorBlueprintResources/StandardMacros.FlipFlop`
      (:`A`
        _)
      (:`B`
        _))
    (`SceneComponent.ToggleVisibility` (`self.SpotLight1`) false)
    (`SceneComponent.ToggleVisibility` (`self.PointLight1`) false)
    (`SceneComponent.ToggleVisibility` (`self.SpotLight`) false)
    (`SceneComponent.ToggleVisibility` (`self.PointLight`) false)
    (`SceneComponent.ToggleVisibility` (`self.PointLight3`) false)
    (`SceneComponent.ToggleVisibility` (`self.PointLight2`) false)))

(event `Key|S`
  (params (Key :type "Key Structure"))
  (:`Pressed`
    (bind (_direction _newtrack_0) (`Timeline|Timeline_0` :!label _label)
      (:`Update`
        (`LightComponent.SetIntensity` (`self.PointLight5`) _newtrack_0)
        (`LightComponent.SetIntensity` (`self.PointLight4`) _newtrack_0))))
  (:`Released`
    (goto _label :!via `Reverse`)))

(event `InputAxis|Drive Forward`
  (params (AxisValue :type "Float (single-precision)"))
  (`WheeledVehicleMovementComponent.SetThrottleInput` (`self.VehicleMovement`) AxisValue))

(event `InputAxis|DriveSteering`
  (params (AxisValue :type "Float (single-precision)"))
  (`WheeledVehicleMovementComponent.SetSteeringInput` (`self.VehicleMovement`) AxisValue))

(fn `GetWeaponSocket`
  (params (SocketName :type Name))
  (returns (SocketTransform :type "Transform Structure"))
  (return))

(fn `UserConstructionScript`)