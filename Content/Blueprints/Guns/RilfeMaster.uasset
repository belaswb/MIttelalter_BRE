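; Base rifle weapon Blueprint that handles firing and exposes socket transforms from its rifle mesh.
; The Fire event spawns a projectile at the Scene component's transform, adds a particle effect at the mesh's "Fire" socket and plays a non-spatialized 2D sound.
; GetWeaponSocket returns the world-space transform of a named socket when the mesh is valid.
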(event `Fire`
  (`|SpawnActorFromClass` "/Game/Blueprints/Guns/Projecil.Projecil_C" (`SceneComponent.K2_GetComponentToWorld` (`self.Scene`)) "Undefined" "OverrideRootScale" null null)
  (`AddComponent|NODE_AddParticleSystemComponent-0` :`RelativeTransform` (`SceneComponent.GetSocketTransform` (`self.SK_Wep_RifleSwat_01`) "Fire" "RTS_Actor"))
  (`GameplayStatics.PlaySound2D` (`self.Sound`) 1.0 1.0 0.0 null null))

(fn `GetWeaponSocket`
  (params (SocketName :type Name))
  (returns (SocketTransform :type "Transform Structure"))
  (bind _sk_wep_rifleswat_01 (`self.SK_Wep_RifleSwat_01`))
  (`/Engine/EditorBlueprintResources/StandardMacros.IsValid` _sk_wep_rifleswat_01
    (:`Is Valid`
      (return (`SceneComponent.GetSocketTransform` _sk_wep_rifleswat_01 SocketName "RTS_World")))))

(fn `UserConstructionScript`)